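; Game instance for a rhythm-based first-person game, judging beat timing and driving enemy and level flow.
; An externally triggered DoBeat opens a hit window, resolves early or late inputs, then tops up, moves and fires enemies.
; During a special attack, each beat teleports the player to the next target to deal multiplier-scaled damage.
; It also changes music pitch and, at song end, saves score, counts kills and opens the score level.
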(event `Setup`
  (bind _asbp_first_person_character (cast `/Game/FirstPerson/Blueprints/BP_FirstPersonCharacter` (`GameplayStatics.GetPlayerCharacter` 0)))
  (set `self.Player` _asbp_first_person_character)
  (`self.TryToSpawn`))

(event `TryToHitBeat`
  ; Beat Check
  (set `self.TriedToHit` true)
  (if (`self.OnBeat`)
    (`/Game/FirstPerson/Blueprints/BP_FirstPersonCharacter.HitSuccess` (`self.Player`))
    (set `self.OnBeatHits` (+ (`self.OnBeatHits`) 1.0))
    (set `self.TriedToHit` false)
    (else
      (set `self.HitBeat` true)
      (`KismetSystemLibrary.Delay` (`self.TimingSpace`))
      (set `self.HitBeat` false)
      (if (`self.TriedToHit`)
        (`/Game/FirstPerson/Blueprints/BP_FirstPersonCharacter.HitFail` (`self.Player`))
        (set `self.TriedToHit` false)
        (`KismetSystemLibrary.PrintText` "I am causing bad and good")))))

(event `SpecialAttack`
  (params (Targets :type "Array of Actor Object Reference"))
  (set `self.Attacking` true)
  (set `self.Targets` Targets)
  (set `self.AttackIndex` 0))

(event `DoBeat`
  (bind _player (`self.Player`))
  (set `self.OnBeat` true)
  ; Beat Check
  (`|ExecutionSequence`
    (:`then_0`
      (if (`self.TriedToHit`)
        (if (`self.HitBeat`)
          (`/Game/FirstPerson/Blueprints/BP_FirstPersonCharacter.HitSuccess` _player)
          (set `self.OnBeatHits` (+ (`self.OnBeatHits`) 1.0))
          (else
            (`/Game/FirstPerson/Blueprints/BP_FirstPersonCharacter.HitFail` _player)))
        (set `self.TriedToHit` false)))
    (:`then_1`
      (`KismetSystemLibrary.Delay` (`self.TimingSpace`))
      (set `self.OnBeat` false))
    (:`then_2`
      (`self.TryToSpawn`)
      (`self.TryToMove`)
      (`self.Enemy Shoot`))
    (:`then_3`
      (if (`self.Attacking`)
        (`self.DashAttack`)))))

(event `TryToSpawn`
  (bind _enemycount (`self.CheckEnemyCount`))
  (if (< _enemycount (`self.EnemyCap`))
    (`/Game/Blueprints/BP_Spawner.Spawn` (`self.Spawner`) (- (`self.EnemyCap`) (`self.EnemyTotal`)))))

(event `TryToMove`
  (for _array_element (`self.Enemies`)
    (`/Engine/EditorBlueprintResources/StandardMacros.IsValid` _array_element
      (:`Is Valid`
        (`/Game/Blueprints/BP_Enemy.RandomRoam` _array_element)))))

(event `DashAttack`
  (bind _player (`self.Player`))
  (bind _player_2 (`self.Player`))
  (bind _player_3 (`self.Player`))
  (bind _output (`|GetArrayItem` (`self.Targets`) (`self.AttackIndex`)))
  (bind _returnvalue (`Actor.K2_GetActorRotation` _output))
  (bind _returnvalue_2 (* (`/Game/FirstPerson/Blueprints/BP_FirstPersonCharacter.Damage` _player) (`/Game/FirstPerson/Blueprints/BP_FirstPersonCharacter.Multiplier` _player) 2.0))
  ; DashAttack
  (if (> (`KismetArrayLibrary.Array_Length` (`self.Targets`)) 0)
    (if (`KismetSystemLibrary.DoesImplementInterface` _output "/Game/Blueprints/BPI_Enemy.BPI_Enemy_C")
      (message `/Game/Blueprints/BPI_Enemy.Unmark` _output)
      (`Actor.K2_SetActorLocation` _player_2 (+ (`Actor.K2_GetActorLocation` _output) (* (`KismetMathLibrary.GetForwardVector` _returnvalue) -30.0)) false true)
      (`Actor.K2_SetActorRotation` _player_2 _returnvalue false)
      (if (> _returnvalue_2 20.0)
        (message `/Game/Blueprints/BPI_Enemy.ReceiveDamage` _output _returnvalue_2)
        (`/Game/FirstPerson/Blueprints/BP_FirstPersonCharacter.ChangeScore` _player_3 (* _returnvalue_2 15.0))
        (else
          (message `/Game/Blueprints/BPI_Enemy.ReceiveDamage` _output 20.0)
          (`/Game/FirstPerson/Blueprints/BP_FirstPersonCharacter.ChangeScore` _player_3 200.0)))
      (bind _output_get (set `self.AttackIndex` (+ (`self.AttackIndex`) 1)))
      (`/Game/FirstPerson/Blueprints/BP_FirstPersonCharacter.AddToMultPercent` _player_3)
      (set `self.SpecialHits` (+ (`self.SpecialHits`) 1.0))
      (if (> _output_get (- (`KismetArrayLibrary.Array_Length` (`self.Targets`)) 1))
        (set `self.Attacking` false)
        (`/Game/FirstPerson/Blueprints/BP_FirstPersonCharacter.FinishSpecialAbility` _player_3)))
    (else
      (set `self.Attacking` false)
      (`/Game/FirstPerson/Blueprints/BP_FirstPersonCharacter.FinishSpecialAbility` _player_2))))

(event `Enemy Shoot`
  (for _array_element (`self.Enemies`)
    (`/Engine/EditorBlueprintResources/StandardMacros.IsValid` _array_element
      (:`Is Valid`
        (`/Game/Blueprints/BP_Enemy.ShootPlayer` _array_element)))))

(event `ChangeMusicSpeed`
  (params (TimeDilation :type "Float (double-precision)"))
  (bind _rhythm (`self.Rhythm`)
    (:`then`
      (`/Game/Blueprints/BP_Rhythm.ChangePitch` _rhythm TimeDilation)
      (`KismetSystemLibrary.PrintText` "ChangingSpeed"))
    (:`else`
      (`KismetSystemLibrary.PrintText` "NotValid"))))

(event `FinishSong`
  (`/Game/FirstPerson/Blueprints/BP_FirstPersonCharacter.FinishLevel` (`self.Player`))
  (`self.SaveScore`)
  (`self.CountKilledEnemies`)
  (`KismetSystemLibrary.Delay` 2.0)
  (`GameplayStatics.OpenLevelBySoftObjectPtr` "/Game/Maps/Score.Score"))

(event `CountKilledEnemies`
  (for _array_element (`self.Enemies`)
    (`/Engine/EditorBlueprintResources/StandardMacros.IsValid` _array_element
      (:`Is Not Valid`
        (set `self.KilledEnemies` (+ (`self.KilledEnemies`) 1)))))
  (`self.KillAllEnemies`))

(event `SaveScore`
  (set `self.Score` (`/Game/FirstPerson/Blueprints/BP_FirstPersonCharacter.Score` (`self.Player`))))

(event `KillAllEnemies`
  (for _array_element (`self.Enemies`)
    (`/Engine/EditorBlueprintResources/StandardMacros.IsValid` _array_element
      (:`Is Valid`
        (`/Game/Blueprints/BP_Enemy.Kill` _array_element))))
  (`KismetArrayLibrary.Array_Clear` (`self.Enemies`)))

(fn `Beat`)

(fn `CheckEnemyCount`
  (returns (EnemyCount :type Integer))
  (set `self.EnemyTotal` 0)
  (for _array_element (`self.Enemies`)
    (`/Engine/EditorBlueprintResources/StandardMacros.IsValid` _array_element
      (:`Is Valid`
        (set `self.EnemyTotal` (+ (`self.EnemyTotal`) 1)))))
  (return (`self.EnemyTotal`)))