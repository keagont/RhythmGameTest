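; Enemy for a rhythm-based game that registers itself in GI_Rhythm's enemy list and starts a random navmesh move on BeginPlay.
; Pawn sensing briefly flags the player as visible, gating ShootPlayer, which turns and fires a bullet on cooldown; nothing here calls it.
; Mark and Unmark toggle a tag and indicator widget.
; Damage swaps materials by health, then at zero clears the list slot, enables mesh physics and destroys the actor after a delay.
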(event `RandomRoam`
  (if (`self.CanMove`)
    (set `self.CanMove` false)
    (bind _randomlocation (`NavigationSystemV1.K2_GetRandomLocationInNavigableRadius` (`SceneComponent.K2_GetComponentLocation` (`self.CapsuleComponent`)) 1000.0 null null))
    (`|AIMoveTo` self _randomlocation null
      (:`OnSuccess`
        _)
      (:`OnFail`
        _))
    (`KismetSystemLibrary.Delay` 2.0)
    (set `self.CanMove` true)))

(event `self.ReceiveBeginPlay`
  (bind _asgi_rhythm (cast `/Game/Blueprints/GI_Rhythm` (`GameplayStatics.GetGameInstance`)))
  (bind _output_get (set `self.GameInstance` _asgi_rhythm))
  (bind _returnvalue (`KismetArrayLibrary.Array_Add` (`/Game/Blueprints/GI_Rhythm.Enemies` _output_get) self))
  (set `self.EnemyIndex` _returnvalue)
  (`self.RandomRoam`))

(event `/Game/Blueprints/BPI_Enemy.Mark`
  (`KismetArrayLibrary.Array_Add` (`self.Tags`) "Marked")
  (bind _returnvalue (`|CreateWidget` "/Game/Blueprints/W_Indicator.W_Indicator_C"))
  (`WidgetComponent.SetWidget` (`self.Indicator`) _returnvalue)
  (`KismetSystemLibrary.PrintText` "Marked!"))

(event `/Game/Blueprints/BPI_Enemy.Unmark`
  (`KismetArrayLibrary.Array_RemoveItem` (`self.Tags`) "Marked")
  (`WidgetComponent.SetWidget` (`self.Indicator`) null))

(event `/Game/Blueprints/BPI_Enemy.ReceiveDamage`
  (params (Damage :type "Float (double-precision)"))
  (bind _mesh (`self.Mesh`))
  (bind _output_get (set `self.Health` (- (`self.Health`) Damage)))
  (`KismetSystemLibrary.PrintText` (`|FormatText` "{health} Health Remaining" _output_get))
  (if (> _output_get 60.0)
    (`PrimitiveComponent.SetMaterial` _mesh 0 "/Game/Blueprints/MI_HighHealth.MI_HighHealth")
    (elif (> _output_get 20.0)
      (`PrimitiveComponent.SetMaterial` _mesh 0 "/Game/Blueprints/MI_MidHealth.MI_MidHealth")
      (elif (> _output_get 0.0)
        (`PrimitiveComponent.SetMaterial` _mesh 0 "/Game/Blueprints/MI_LowHealth.MI_LowHealth")
        (else
          (set `self.Health` 0.0)
          (`KismetArrayLibrary.Array_Set` (`/Game/Blueprints/GI_Rhythm.Enemies` (`self.GameInstance`)) (`self.EnemyIndex`))
          (`PrimitiveComponent.SetSimulatePhysics` (`self.Mesh`) true)
          (`KismetSystemLibrary.Delay` 5.0)
          (`self.K2_DestroyActor` :!label _label))))))

(event `Kill`
  (goto _label))

(event `ShootPlayer`
  (bind (_returnvalue_location _returnvalue_rotation) (`KismetMathLibrary.BreakTransform` (`self.GetTransform`)))
  (if (and (`self.CanSeePlayer`) (`self.CanShoot`))
    (set `self.CanShoot` false)
    (bind _asbp_first_person_character (cast `/Game/FirstPerson/Blueprints/BP_FirstPersonCharacter` (`GameplayStatics.GetPlayerCharacter` 0)))
    (`self.K2_SetActorRotation` (`KismetMathLibrary.FindLookAtRotation` (`self.K2_GetActorLocation`) (`self.K2_GetActorLocation` _asbp_first_person_character)))
    (`|SpawnActorFromClass` "/Game/Blueprints/BP_Bullet.BP_Bullet_C" (`KismetMathLibrary.MakeTransform` (+ (* (`KismetMathLibrary.GetForwardVector` _returnvalue_rotation) 20.0) _returnvalue_location) _returnvalue_rotation) "Undefined" "MultiplyWithRoot" null null)
    (`KismetSystemLibrary.Delay` (`self.ShootCooldown`))
    (set `self.CanShoot` true)))

(event `self.PawnSensing.OnSeePawn`
  (params (Pawn :type "Pawn Object Reference"))
  (cast `/Game/FirstPerson/Blueprints/BP_FirstPersonCharacter` Pawn)
  (set `self.CanSeePlayer` true)
  (`KismetSystemLibrary.RetriggerableDelay` 2.0)
  (set `self.CanSeePlayer` false))

(fn `UserConstructionScript`)