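; BP_Rhythm is the music conductor actor that plays the test song and drives the game's beat and song-end events through GI_Rhythm.
; It registers itself on the game instance at BeginPlay, and SyncMusic spawns the MetaSound as 2D audio.
; MetaSound output watchers turn the beat and finish outputs into DoBeat and a delayed FinishSong call on the game instance.
; ChangePitch sets the song's speed parameter.
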(event `self.ReceiveBeginPlay`
  (bind _asgi_rhythm (cast `/Game/Blueprints/GI_Rhythm` (`GameplayStatics.GetGameInstance`)))
  (bind _output_get (set `self.GameInstance` _asgi_rhythm))
  (set `/Game/Blueprints/GI_Rhythm.Rhythm` self _output_get)
  (bind _asbp_first_person_character (cast `/Game/FirstPerson/Blueprints/BP_FirstPersonCharacter` (`GameplayStatics.GetPlayerCharacter` 0)))
  (set `self.Player` _asbp_first_person_character))

(event `ChangePitch`
  (params (Pitch :type "Float (double-precision)"))
  (`AudioParameterControllerInterface.SetFloatParameter` (`self.Song`) "speed" Pitch)
  (`KismetSystemLibrary.PrintText` (`|FormatText` "Changed speed to {speed}" Pitch)))

(event `SyncMusic`
  (bind _returnvalue (`GameplayStatics.SpawnSound2D` "/Game/Audio/MSS_TestGameMusic.MSS_TestGameMusic" 1.0 1.0 0.0 null))
  (bind _output_get (set `self.Song` _returnvalue))
  (`MetaSoundOutputSubsystem.WatchOutput` (subsystem `MetaSoundOutputSubsystem`) _output_get "TestOnBeat" (delegate `SongBeat`) "None" "None")
  (`MetaSoundOutputSubsystem.WatchOutput` (subsystem `MetaSoundOutputSubsystem`) _output_get "FinishSong" (delegate `Finish Song`) "None" "None"))

(event `SongBeat`
  (params (OutputName :type Name) (Output :type "MetaSoundOutput Structure (by ref)"))
  (`/Game/Blueprints/GI_Rhythm.DoBeat` (`self.GameInstance`))
  (`KismetSystemLibrary.PrintText` "SYNC MUSIC" true true (struct :`R` 0.050557 :`G` 0.050011 :`B` 1.0 :`A` 1.0) 0.5))

(event `Finish Song`
  (params (OutputName :type Name) (Output :type "MetaSoundOutput Structure (by ref)"))
  (`KismetSystemLibrary.PrintText` "SONG FINISHED" true true (struct :`R` 1.0 :`B` 0.027063 :`A` 1.0) 10.0)
  (`KismetSystemLibrary.Delay` 1.0)
  (`/Game/Blueprints/GI_Rhythm.FinishSong` (`self.GameInstance`)))

(fn `UserConstructionScript`)